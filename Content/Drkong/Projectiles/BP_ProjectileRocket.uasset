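; BP_ProjectileRocket is a rocket projectile built to fly a randomized curved path to a target location.
; On Tick, behind a gate, a control point slides toward the target while the rocket chases it at the same speed, facing the target.
; Helper functions place that point randomly along the line, offset sideways and rotated around it.
; The launch setup (target capture, muzzle flash, curve calculation, gate opening) is disconnected and never runs.
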(event `self.ReceiveTick`
  (params (DeltaSeconds :type "Float (single-precision)"))
  (`/Engine/EditorBlueprintResources/StandardMacros.Gate` true
    (:`Exit`
      (if (!= (`self.K2_GetActorLocation`) (`self.TargetLocation`))
        (set `self.Curved Point` (`KismetMathLibrary.VInterpTo_Constant` (`self.Curved Point`) (`self.TargetLocation`) (`GameplayStatics.GetWorldDeltaSeconds`) (`self.Speed`)))
        (`self.K2_SetActorLocationAndRotation` (`KismetMathLibrary.VInterpTo_Constant` (`self.K2_GetActorLocation`) (`self.Curved Point`) (`GameplayStatics.GetWorldDeltaSeconds`) (`self.Speed`)) (`KismetMathLibrary.FindLookAtRotation` (`self.K2_GetActorLocation`) (`self.TargetLocation`)))))))

(event `self.ReceiveBeginPlay`)

(fn `Curve Control Point`
  (bind (_x _y) (`KismetMathLibrary.BreakRotIntoAxes` (`KismetMathLibrary.FindLookAtRotation` (`self.Mid Point`) (`self.TargetLocation`))))
  (set `self.Curved Point` (+ (`self.Mid Point`) (`KismetMathLibrary.RotateAngleAxis` (* (`KismetMathLibrary.RandomFloatInRange` (`self.Min Curve Radius`) (`self.Max Curve Radius`)) _y) (`KismetMathLibrary.RandomFloatInRange` (`self.Min Angle`) (`self.Max Angle`)) _x))))

(fn `Mid Point Calculator`
  (set `self.Mid Point` (+ (* (- (`self.TargetLocation`) (`self.K2_GetActorLocation`)) (`KismetMathLibrary.RandomFloatInRange` (`self.Min Curve Point Distance`) (`self.Max Curve Point Distance`))) (`self.K2_GetActorLocation`))))

(fn `UserConstructionScript`
  (`parent.UserConstructionScript`))