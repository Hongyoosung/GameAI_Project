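; AI controller for an agent that senses nearby Wraith player characters and drives its pawn's StateMachine component.
; Shortly after BeginPlay it caches the component's Attack, MoveTo, Flee and Dead states, though only Attack is used here.
; Perception updates sort characters into allies (team hard-coded as 1) or enemies, and an enemy switches the machine to Attack.
; Tick prunes both lists of anyone beyond SurroundRadius, removing entries while iterating.
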(event OnPerceptionUpdated(AIPerception)
  (params (UpdatedActors :type Array%20of%20Actor%20Object%20References))
  (for _array_element UpdatedActors
    (bind _aswraith_player_character (Utilities|Casting|CastToWraithPlayerCharacter _array_element))
    (bind _output_get (Variables|Default|SetFoundUnit _aswraith_player_character))
    (bind _team_number (Class|BPIDamageable|GetTeamNumber(Message) _output_get))
    (if (== 1 _team_number)
      (Utilities|Array|Add (Variables|Default|GetSurroundAlies) (Variables|Default|GetFoundUnit))
      (Development|PrintString "Find Alies")
      (else
        (Utilities|Array|Add (Variables|Default|GetSurroundEnemies) (Variables|Default|GetFoundUnit))
        (Development|PrintString "Find Enemy")
        (Class|StateMachine|ChangeState (Variables|Default|GetStateMachine) (Variables|Default|GetAttack%20State))))))

(event EventBeginPlay
  (Variables|Default|SetStateMachine (Actor|GetComponentbyClass (Pawn|GetControlledPawn) "/Script/GameAI_Project.StateMachine"))
  (Utilities|FlowControl|Delay 1.0)
  (Utilities|FlowControl|Sequence
    (:then_0
      (bind _returnvalue (Class|StateMachine|GetAttackState (Variables|Default|GetStateMachine)))
      (Variables|Default|SetAttack%20State _returnvalue))
    (:then_1
      (bind _returnvalue_2 (Class|StateMachine|GetMovetoState (Variables|Default|GetStateMachine)))
      (Variables|Default|SetMoveTo%20State _returnvalue_2))
    (:then_2
      (bind _returnvalue_3 (Class|StateMachine|GetFleeState (Variables|Default|GetStateMachine)))
      (Variables|Default|SetFlee%20State _returnvalue_3))
    (:then_3
      (bind _returnvalue_4 (Class|StateMachine|GetDeadState (Variables|Default|GetStateMachine)))
      (Variables|Default|SetDead%20State _returnvalue_4))))

(event EventTick
  (params (DeltaSeconds :type Float%20%28single-precision%29))
  (Utilities|FlowControl|Sequence
    (:then_0
      (for _array_element (Variables|Default|GetSurroundEnemies)
        (if (> (Transformation|GetDistanceTo _array_element) (Variables|Default|GetSurroundRadius))
          (Utilities|Array|RemoveItem (Variables|Default|GetSurroundEnemies) _array_element))))
    (:then_1
      (for _array_element_2 (Variables|Default|GetSurroundAlies)
        (if (> (Transformation|GetDistanceTo _array_element_2) (Variables|Default|GetSurroundRadius))
          (Utilities|Array|RemoveItem (Variables|Default|GetSurroundAlies) _array_element_2))))))

(fn ConstructionScript)

(fn SetStateasAttack)

(fn GetFoundUnit
  (return (Variables|Default|GetFoundUnit)))