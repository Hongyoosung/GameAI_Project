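; AI controller for an agent that tracks surrounding allies and enemies and switches its pawn's StateMachine component between states.
; After a short delay on BeginPlay it caches attack, move, flee and dead states and binds death events on listed enemies.
; External callers update the lists and trigger move or attack changes through events.
; Perception sorting by team, radius pruning and automatic state selection are present but unwired, leaving Tick empty.
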(event OnPerceptionUpdated(AIPerception)
  (params (UpdatedActors :type Array%20of%20Actor%20Object%20References)))

(event Custom|Change%20MoveTo
  (Class|StateMachine|ChangeState (Variables|Default|GetStateMachine) (Variables|Default|GetMoveTo%20State)))

(event Custom|Remove%20enemy
  (bind _surroundalies (Variables|Default|GetSurroundAlies))
  (bind _surroundenemies (Variables|Default|GetSurroundEnemies))
  (bind _team_number (Class|BPIDamageable|GetTeamNumber(Message) (stale EventBeginPlay _aswraith_player_character)))
  (bind _team_number_2 (Class|BPIDamageable|GetTeamNumber(Message) (Pawn|GetControlledPawn)))
  (if (!= _team_number _team_number_2)
    (Utilities|Array|RemoveIndex _surroundenemies (- (Utilities|Array|Length _surroundenemies) 1))
    (else
      (Utilities|Array|RemoveIndex _surroundalies (- (Utilities|Array|Length _surroundalies) 1)))))

(event Custom|Change%20Attack
  (Class|StateMachine|ChangeState (Variables|Default|GetStateMachine) (Variables|Default|GetAttack%20State)))

(event EventBeginPlay
  (Variables|Default|SetStateMachine (Actor|GetComponentbyClass (Pawn|GetControlledPawn) "/Script/GameAI_Project.StateMachine"))
  (Utilities|FlowControl|Delay 1.0)
  (Utilities|FlowControl|Sequence
    (:then_0
      (bind _returnvalue (Class|StateMachine|GetAttackState (Variables|Default|GetStateMachine)))
      (Variables|Default|SetAttack%20State _returnvalue))
    (:then_1
      (bind _returnvalue_2 (Class|StateMachine|GetMovetoState (Variables|Default|GetStateMachine)))
      (Variables|Default|SetMoveTo%20State _returnvalue_2))
    (:then_2
      (bind _returnvalue_3 (Class|StateMachine|GetFleeState (Variables|Default|GetStateMachine)))
      (Variables|Default|SetFlee%20State _returnvalue_3))
    (:then_3
      (bind _returnvalue_4 (Class|StateMachine|GetDeadState (Variables|Default|GetStateMachine)))
      (Variables|Default|SetDead%20State _returnvalue_4))
    (:then_5
      (for _array_element (Variables|Default|GetSurroundEnemies)
        (bind _aswraith_player_character (Utilities|Casting|CastToWraithPlayerCharacter _array_element))
        (EventDispatchers|BindEventtoDead _aswraith_player_character (delegate Custom|Remove%20enemy))))))

(event EventTick
  (params (DeltaSeconds :type Float%20%28single-precision%29))
  (Utilities|FlowControl|Sequence))

(event EventAddSurroundAlies
  (params (Ally :type Wraith%20Player%20Character%20Object%20Reference))
  (Utilities|Array|Add (Variables|Default|GetSurroundAlies) Ally))

(event EventAddSurroundEnemies
  (params (Enemy :type Wraith%20Player%20Character%20Object%20Reference))
  (Utilities|Array|Add (Variables|Default|GetSurroundEnemies) Enemy))

(event EventSubSurrondAlies
  (params (Ally :type Wraith%20Player%20Character%20Object%20Reference))
  (Utilities|Array|RemoveItem (Variables|Default|GetSurroundEnemies) Ally))

(event EventSubSurrondEnemies
  (params (Enemy :type Wraith%20Player%20Character%20Object%20Reference))
  (Utilities|Array|RemoveItem (Variables|Default|GetSurroundEnemies) Enemy))

(fn ConstructionScript)

(fn SetStateasAttack)

(fn GetFoundUnit
  (return (Variables|Default|GetFoundUnit)))

(fn GetSurroundAlies
  (return (Variables|Default|GetSurroundAlies)))

(fn GetSurroundAliesNum
  (return (Utilities|Array|Length (Variables|Default|GetSurroundAlies))))

(fn GetSurroundEnemies
  (return (Variables|Default|GetSurroundEnemies)))

(fn GetSurroundEnemiesNum
  (return (Utilities|Array|Length (Variables|Default|GetSurroundEnemies))))